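; BP_TracksReverse is a train-track ground segment that spawns trains and helps extend the level as the player crosses it.
; Tick runs a countdown through UpdateCars and CheckSpawnTimer; on expiry, SpawnCars randomly decides whether to spawn BP_Trains at a fixed Y position.
; Player overlap with SpawnNewZone asks TrackSpawner for new ground, while TriggerZone destroys the segment.
; Older car-spawning logic remains disconnected, despite the car-based function names.
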(event OnComponentBeginOverlap(TriggerZone)
  (params (OverlappedComponent :type Primitive%20Component%20Object%20Reference) (OtherActor :type Actor%20Object%20Reference) (OtherComp :type Primitive%20Component%20Object%20Reference) (OtherBodyIndex :type Integer) (bFromSweep :type Boolean) (SweepResult :type Hit%20Result%20Structure%20%28by%20ref%29))
  (Utilities|Casting|CastToBP_Player OtherActor)
  (Actor|DestroyActor))

(event OnComponentBeginOverlap(CarZone)
  (params (OverlappedComponent :type Primitive%20Component%20Object%20Reference) (OtherActor :type Actor%20Object%20Reference) (OtherComp :type Primitive%20Component%20Object%20Reference) (OtherBodyIndex :type Integer) (bFromSweep :type Boolean) (SweepResult :type Hit%20Result%20Structure%20%28by%20ref%29)))

(event OnComponentBeginOverlap(SpawnNewZone)
  (params (OverlappedComponent :type Primitive%20Component%20Object%20Reference) (OtherActor :type Actor%20Object%20Reference) (OtherComp :type Primitive%20Component%20Object%20Reference) (OtherBodyIndex :type Integer) (bFromSweep :type Boolean) (SweepResult :type Hit%20Result%20Structure%20%28by%20ref%29))
  (bind _trackspawner (Variables|Default|GetTrackSpawner))
  (Utilities|Casting|CastToBP_Player OtherActor)
  (Utilities|IsValid _trackspawner
    (:Is%20Valid
      (Default|SpawnGroundatSpawnPoint _trackspawner))))

(event EventBeginPlay)

(event EventTick
  (params (DeltaSeconds :type Float%20%28single-precision%29))
  (CallFunction|UpdateCars))

(event Collision|EventActorBeginOverlap
  (params (OtherActor :type Actor%20Object%20Reference))
  ;[1 1 1] Old Stuff, may reuse
)

(fn ConstructionScript)

(fn CheckSpawnTimer
  (Variables|Default|SetSpawnTimer (- (Variables|Default|GetSpawnTimer) (Utilities|Time|GetWorldDeltaSeconds)))
  (if (<= (Variables|Default|GetSpawnTimer) 0.0)
    (Variables|Default|SetSpawnTimer (Variables|Default|GetDurationBetweenSpawn))
    (CallFunction|SpawnCars)))

(fn SpawnCars
  (bind _returnvalue (Transformation|GetActorLocation))
  (bind _returnvalue_2 (Math|Random|RandomIntegerinRange 0 10))
  (if (and (>= _returnvalue_2 0) (< _returnvalue_2 7))
    (Game|SpawnActorfromClass "/Game/Blueprints/BP_Trains.BP_Trains_C" (Math|Transform|MakeTransform (Math|Vector|MakeVector (- (.x _returnvalue) 25.0) -3.5e+03 (+ (.z _returnvalue) 75.0)) "0, 0, 0" "1,1,1") "Undefined" 0 0)))

(fn UpdateCars
  (CallFunction|CheckSpawnTimer))