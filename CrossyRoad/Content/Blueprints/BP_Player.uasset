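; Player pawn for a Crossy Road-style hopper that moves through lanes of cars, trains and water lilies.
; Input calls hop functions that rotate, lift and add movement input, which Tick consumes as a swept offset, with sideways bounds and step counting.
; Idling or backing up too far triggers death with eagle sound and restart widget.
; Hitting vehicles or lilies disables collision; RestartGame restores it, resets position and respawns starting ground.
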(event EventBeginPlay
  (bind _returnvalue (UserInterface|CreateWidget "/Game/UI/WBP_Restart.WBP_Restart_C"))
  (Variables|Default|SetRestartWiget _returnvalue)
  (bind _returnvalue_2 (UserInterface|CreateWidget "/Game/UI/BP_HUD.BP_HUD_C"))
  (bind _output_get (Variables|Default|SetBP_HUD _returnvalue_2))
  (UserInterface|Viewport|AddtoViewport _output_get 0))

(event Collision|EventActorBeginOverlap
  (params (OtherActor :type Actor%20Object%20Reference)))

(event EventTick
  (params (DeltaSeconds :type Float%20%28single-precision%29))
  (if (not (Variables|Default|GetisDead))
    (if (Variables|Default|Getismoving)
      (Variables|Default|SetspawnTimer 6.0)
      (bind _returnvalue (Class|Pawn|ConsumeMovementInputVector :!label _label))
      (Transformation|AddActorLocalOffset _returnvalue true false)
      (else
        (bind _output_get (Variables|Default|SetspawnTimer (- (Variables|Default|GetspawnTimer) (Utilities|Time|GetWorldDeltaSeconds))))
        (if (<= _output_get 0.0)
          (Variables|Default|SetspawnTimer (Variables|Default|Getdurantion))
          (Variables|Default|SetisDead true)
          (CallFunction|DisplayRestart)
          (Variables|Default|SetRestartShowing true)
          (Audio|PlaySoundatLocation "/Game/Blueprints/sounds/eaglesounds.eaglesounds" (Variables|Default|Getplayervec) "0, 0, 0" 1.0 1.0 0.0 0 0 0)
          (else
            (goto _label)))))))

(event Collision|EventHit
  (params (MyComp :type Primitive%20Component%20Object%20Reference) (Other :type Actor%20Object%20Reference) (OtherComp :type Primitive%20Component%20Object%20Reference) (bSelfMoved :type Boolean) (HitLocation :type Vector :default "0, 0, 0") (HitNormal :type Vector :default "0, 0, 0") (NormalImpulse :type Vector :default "0, 0, 0") (Hit :type Hit%20Result%20Structure%20%28by%20ref%29))
  (Utilities|FlowControl|Sequence
    (:then_0
      (Utilities|Casting|CastToBP_Cars Other)
      (Collision|SetCollisionEnabled MyComp "NoCollision"))
    (:then_1
      (Utilities|Casting|CastToBP_CarsReverse Other)
      (Collision|SetCollisionEnabled MyComp "NoCollision"))
    (:then_2
      (Utilities|Casting|CastToBP_Trains Other)
      (Collision|SetCollisionEnabled MyComp "NoCollision"))
    (:then_3
      (Utilities|Casting|CastToBP_TrainsReverse Other)
      (Collision|SetCollisionEnabled MyComp "NoCollision"))
    (:then_4
      (Utilities|Casting|CastToBP_WaterLillies Other)
      (Collision|SetCollisionEnabled MyComp "NoCollision"))))

(event Input|ActionEvents|InputActionMoveForward
  (params (Key :type Key%20Structure))
  ;[1 1 1] Player Movement
  (:Pressed
    (CallFunction|MoveFo)
    (Variables|Default|Setismoving true)
    (Audio|PlaySoundatLocation "/Game/Blueprints/sounds/stepsound_Cue.stepsound_Cue" (Variables|Default|Getplayervec) "0, 0, 0" 1.0 1.0 0.0 0 0 0))
  (:Released
    (Variables|Default|Setismoving false)))

(event Input|ActionEvents|InputActionMoveBackward
  (params (Key :type Key%20Structure))
  ;[1 1 1] Player Movement
  (:Pressed
    (CallFunction|MoveBa)
    (if (== (Variables|Default|GetBackupSteps) -5)
      (Variables|Default|SetisDead true)
      (CallFunction|DisplayRestart)
      (Variables|Default|SetRestartShowing true)
      (Audio|PlaySoundatLocation "/Game/Blueprints/sounds/eaglesounds.eaglesounds" (Variables|Default|Getplayervec) "0, 0, 0" 1.0 1.0 0.0 0 0 0)
      (else
        (Audio|PlaySoundatLocation "/Game/Blueprints/sounds/stepsound_Cue.stepsound_Cue" (Variables|Default|Getplayervec) "0, 0, 0" 1.0 1.0 0.0 0 0 0)))))

(event Input|ActionEvents|InputActionMoveRight
  (params (Key :type Key%20Structure))
  ;[1 1 1] Player Movement
  (:Pressed
    (if (not (> (.y (Transformation|GetActorLocation)) 2e+03))
      (CallFunction|MoveRi)
      (Audio|PlaySoundatLocation "/Game/Blueprints/sounds/stepsound_Cue.stepsound_Cue" (Variables|Default|Getplayervec) "0, 0, 0" 1.0 1.0 0.0 0 0 0))))

(event Input|ActionEvents|InputActionMoveLeft
  (params (Key :type Key%20Structure))
  ;[1 1 1] Player Movement
  (:Pressed
    (if (not (< (.y (Transformation|GetActorLocation)) -1e+03))
      (CallFunction|MoveLe)
      (Audio|PlaySoundatLocation "/Game/Blueprints/sounds/stepsound_Cue.stepsound_Cue" (Variables|Default|Getplayervec) "0, 0, 0" 1.0 1.0 0.0 0 0 0))))

(fn ConstructionScript)

(fn DisplayRestart
  (bind _returnvalue (Game|GetPlayerController 0))
  (UserInterface|Viewport|AddtoViewport (Variables|Default|GetRestartWiget) 0)
  (Input|SetInputModeUIOnly _returnvalue 0 "DoNotLock")
  (Variables|/Script/Engine.PlayerController|SetbShowMouseCursor _returnvalue true))

(fn RestartGame
  (bind _returnvalue (Game|GetPlayerController 0))
  (Variables|Default|SetisDead false)
  (Widget|RemovefromParent (Variables|Default|GetRestartWiget))
  (Input|SetInputModeGameOnly _returnvalue)
  (Variables|/Script/Engine.PlayerController|SetbShowMouseCursor _returnvalue false)
  (Transformation|SetActorLocation "0.000000,216.000000,200.000000" false false)
  (Collision|SetCollisionEnabled (Variables|Default|GetBox) "QueryAndPhysics")
  (Default|SpawnInitialGrounds (Variables|Default|GetNewVar_0)))

(fn MoveFo
  (bind _returnvalue (Transformation|GetActorForwardVector))
  (bind _returnvalue_2 (* _returnvalue -1.0))
  (Transformation|SetActorRotation "0,90.000000,0.000000")
  (Transformation|AddActorLocalOffset (Math|Vector|MakeVector (.x _returnvalue_2) (.y _returnvalue_2) 4e+01) false false)
  (Pawn|Input|AddMovementInput (Math|Vector|MakeVector (.x _returnvalue_2) (.y _returnvalue_2) (.z _returnvalue_2)) (Variables|Default|GetHopDist) false)
  (if (< (Variables|Default|GetBackupSteps) (Variables|Default|GetSteps))
    (Math|Integer|IncrementInt (Variables|Default|GetBackupSteps))
    (else
      (bind _result (Math|Integer|IncrementInt (Variables|Default|GetSteps))
        (:%20%20
          (Variables|Default|SetBackupSteps _result))))))

(fn MoveBa
  (bind _returnvalue (Transformation|GetActorForwardVector))
  (Transformation|SetActorRotation "0,-90.000000,0.000000")
  (Transformation|AddActorLocalOffset (Math|Vector|MakeVector (.x _returnvalue) (.y _returnvalue) 4e+01) false false)
  (Pawn|Input|AddMovementInput (Math|Vector|MakeVector (.x _returnvalue) (.y _returnvalue) (.z _returnvalue)) (Variables|Default|GetHopDist) false)
  (Math|Integer|DecrementInt (Variables|Default|GetBackupSteps)))

(fn MoveLe
  (bind _returnvalue (Transformation|GetActorRightVector))
  (Transformation|SetActorRotation "0, 0, 0")
  (Transformation|AddActorLocalOffset (Math|Vector|MakeVector (.x _returnvalue) (.y _returnvalue) 4e+01) false false)
  (Pawn|Input|AddMovementInput (Math|Vector|MakeVector (.x _returnvalue) (.y _returnvalue) (.z _returnvalue)) (* (Variables|Default|GetHopDist) -1.0) false))

(fn MoveRi
  (bind _returnvalue (Transformation|GetActorRightVector))
  (bind _returnvalue_2 (* _returnvalue -1.0))
  (Transformation|SetActorRotation "0,180.000000, 0")
  (Transformation|AddActorLocalOffset (Math|Vector|MakeVector (.x _returnvalue_2) (.y _returnvalue_2) 4e+01) false false)
  (Pawn|Input|AddMovementInput (Math|Vector|MakeVector (.x _returnvalue_2) (.y _returnvalue_2) (.z _returnvalue_2)) (* (Variables|Default|GetHopDist) -1.0) false))