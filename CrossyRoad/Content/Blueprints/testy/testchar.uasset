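; Test player character for hop-style movement, where each directional input press snaps the actor's yaw and adds movement input scaled by HopDist.
; Only forward also jumps, with OnJumped adding a swept local offset.
; Forward and backward presses adjust BackupSteps, and Steps increments only when forward passes its previous high.
; HUD and restart widget creation and car-hit collision disabling are disconnected and never run.
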(event EventBeginPlay)

(event Collision|EventActorBeginOverlap
  (params (OtherActor :type Actor%20Object%20Reference)))

(event EventTick
  (params (DeltaSeconds :type Float%20%28single-precision%29))
  (if true
    _))

(event EventOnJumped
  (bind _playervec (Variables|Default|Getplayervec))
  (Transformation|AddActorLocalOffset (Math|Vector|MakeVector (+ (.x _playervec) 1.5e+02) (.y _playervec) (.z _playervec)) true false))

(event Collision|EventHit
  (params (MyComp :type Primitive%20Component%20Object%20Reference) (Other :type Actor%20Object%20Reference) (OtherComp :type Primitive%20Component%20Object%20Reference) (bSelfMoved :type Boolean) (HitLocation :type Vector :default "0, 0, 0") (HitNormal :type Vector :default "0, 0, 0") (NormalImpulse :type Vector :default "0, 0, 0") (Hit :type Hit%20Result%20Structure%20%28by%20ref%29)))

(event Input|ActionEvents|InputActionMoveForward
  (params (Key :type Key%20Structure))
  ;[1 1 1] Player Movement
  (:Pressed
    (Transformation|SetActorRotation "0,90.000000, 0")
    (Character|Jump)
    (Pawn|Input|AddMovementInput (* (Transformation|GetActorForwardVector) -1.0) (Variables|Default|GetHopDist) false)
    (if (< (Variables|Default|GetBackupSteps) (Variables|Default|GetSteps))
      (Math|Integer|IncrementInt (Variables|Default|GetBackupSteps))
      (else
        (bind _result (Math|Integer|IncrementInt (Variables|Default|GetSteps))
          (:%20%20
            (Variables|Default|SetBackupSteps _result)
            (Development|PrintString (Utilities|String|ToString(Float) (.z (Variables|Default|Getplayervec))))))))))

(event Input|ActionEvents|InputActionMoveBackward
  (params (Key :type Key%20Structure))
  ;[1 1 1] Player Movement
  (:Pressed
    (Transformation|SetActorRotation "0,-90.000000,0.000000")
    (Pawn|Input|AddMovementInput (Transformation|GetActorForwardVector) (Variables|Default|GetHopDist) false)
    (Math|Integer|DecrementInt (Variables|Default|GetBackupSteps))))

(event Input|ActionEvents|InputActionMoveRight
  (params (Key :type Key%20Structure))
  ;[1 1 1] Player Movement
  (:Pressed
    (Transformation|SetActorRotation "0,180.000000, 0")
    (Pawn|Input|AddMovementInput (* (Transformation|GetActorRightVector) -1.0) (* (Variables|Default|GetHopDist) -1.0) false)))

(event Input|ActionEvents|InputActionMoveLeft
  (params (Key :type Key%20Structure))
  ;[1 1 1] Player Movement
  (:Pressed
    (Transformation|SetActorRotation "0, 0, 0")
    (Pawn|Input|AddMovementInput (Transformation|GetActorRightVector) (* (Variables|Default|GetHopDist) -1.0) false)))

(fn ConstructionScript)