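; Spawns a lane-based level of randomly chosen ground and hazard strips along the X axis.
; On BeginPlay it destroys existing BP_Ground actors, seeds one if none is valid, then fills out an initial run of strips.
; SpawnGround randomly picks one of three ground variants or calls SpawnHazards for roads, water, lilies or tracks, most with reverse variants.
; Each spawn advances a shared TestSpawnPoint and hands the new actor a spawner reference.
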(event EventBeginPlay
  (CallFunction|SpawnInitialGrounds))

(event Collision|EventActorBeginOverlap
  (params (OtherActor :type Actor%20Object%20Reference)))

(event EventTick
  (params (DeltaSeconds :type Float%20%28single-precision%29)))

(fn ConstructionScript)

(fn SpawnGround
  (params (SpawnLocation :type Vector))
  (bind _returnvalue (Math|Random|RandomIntegerinRange 0 2))
  (if (>= (Math|Random|RandomIntegerinRange 0 42) 17)
    (if (== _returnvalue 0)
      (CallFunction|SpawnGroundDefault)
      (elif (== _returnvalue 1)
        (CallFunction|SpawnGround2)
        (else
          (CallFunction|SpawnGround3))))
    (else
      (CallFunction|SpawnHazards))))

(fn SpawnGroundatSpawnPoint
  (CallFunction|SpawnGround (Variables|Default|GettestSpawnPoint)))

(fn SpawnInitialGrounds
  (Utilities|FlowControl|Sequence
    (:then_0
      (bind _outactors (Actor|GetAllActorsOfClass "/Game/Blueprints/BP_Ground.BP_Ground_C"))
      (for _array_element _outactors
        (Actor|DestroyActor _array_element)))
    (:then_1
      (for _index (range 0 24)
        (Utilities|IsValid (Variables|Default|GetNewestGround)
          (:Is%20Valid
            (CallFunction|SpawnGroundatSpawnPoint))
          (:Is%20Not%20Valid
            (bind _returnvalue (Game|SpawnActorfromClass "/Game/Blueprints/BP_Ground.BP_Ground_C" (Math|Transform|MakeTransform (Variables|Default|GettestSpawnPoint) "0, 0, 0" "1,1,1") "Undefined" 0 0))
            (bind _output_get (Variables|Default|SetNewestGround _returnvalue))
            (Variables|/Game/Blueprints/BP_Ground.BP_Ground_C|SetGroundSpawner _output_get self)
            (Variables|Default|SettestSpawnPoint (Math|Vector|MakeVector (+ (.x (Variables|Default|GettestSpawnPoint)) 1.5e+02) (.y (Variables|Default|GettestSpawnPoint)) (.z (Variables|Default|GettestSpawnPoint))))))))))

(fn SpawnRoadatSpawnPoint
  (bind _newestroad (Variables|Default|GetNewestRoad))
  (bind _spawnpoint (Variables|/Game/Blueprints/BP_Road.BP_Road_C|GetSpawnPoint _newestroad))
  (bind _returnvalue (Transformation|GetWorldLocation _spawnpoint))
  (CallFunction|SpawnRoad (Math|Vector|MakeVector (.x _returnvalue) (.y _returnvalue) -75.0)))

(fn SpawnRoad
  (params (SpawnLoc :type Vector))
  (bind _returnvalue (Game|SpawnActorfromClass "/Game/Blueprints/BP_Road.BP_Road_C" (Math|Transform|MakeTransform (Math|Vector|MakeVector (+ (.x SpawnLoc) 0.0) (- (.y SpawnLoc) 1e+03) (- (.z SpawnLoc) 7e+01)) "0, 0, 0" "1,1,1") "Undefined" 0 0))
  (Variables|/Game/Blueprints/BP_Road.BP_Road_C|SetRoadSpawner _returnvalue self)
  (Variables|Default|SettestSpawnPoint (Math|Vector|MakeVector (+ (.x (Variables|Default|GettestSpawnPoint)) 1.5e+02) (.y (Variables|Default|GettestSpawnPoint)) (.z (Variables|Default|GettestSpawnPoint)))))

(fn SpawnGround2
  (bind _returnvalue (Game|SpawnActorfromClass "/Game/Blueprints/BP_Ground2.BP_Ground2_C" (Math|Transform|MakeTransform (Math|Vector|MakeVector (.x (Variables|Default|GettestSpawnPoint)) (.y (Variables|Default|GettestSpawnPoint)) (.z (Variables|Default|GettestSpawnPoint))) "0, 0, 0" "1,1,1") "Undefined" 0 0))
  (bind _output_get (Variables|Default|SetNewestGround2 _returnvalue))
  (Variables|/Game/Blueprints/BP_Ground2.BP_Ground2_C|SetGround2Spawner _output_get self)
  (Variables|Default|SettestSpawnPoint (Math|Vector|MakeVector (+ (.x (Variables|Default|GettestSpawnPoint)) 1.5e+02) (.y (Variables|Default|GettestSpawnPoint)) (.z (Variables|Default|GettestSpawnPoint)))))

(fn SpawnGround3
  (bind _returnvalue (Game|SpawnActorfromClass "/Game/Blueprints/BP_Ground3.BP_Ground3_C" (Math|Transform|MakeTransform (Math|Vector|MakeVector (.x (Variables|Default|GettestSpawnPoint)) (.y (Variables|Default|GettestSpawnPoint)) (.z (Variables|Default|GettestSpawnPoint))) "0, 0, 0" "1,1,1") "Undefined" 0 0))
  (bind _output_get (Variables|Default|SetNewestGround3 _returnvalue))
  (Variables|/Game/Blueprints/BP_Ground3.BP_Ground3_C|SetGround3Spawner _output_get self)
  (Variables|Default|SettestSpawnPoint (Math|Vector|MakeVector (+ (.x (Variables|Default|GettestSpawnPoint)) 1.5e+02) (.y (Variables|Default|GettestSpawnPoint)) (.z (Variables|Default|GettestSpawnPoint)))))

(fn SpawnGroundDefault
  (bind _returnvalue (Game|SpawnActorfromClass "/Game/Blueprints/BP_Ground.BP_Ground_C" (Math|Transform|MakeTransform (Math|Vector|MakeVector (.x (Variables|Default|GettestSpawnPoint)) (.y (Variables|Default|GettestSpawnPoint)) (.z (Variables|Default|GettestSpawnPoint))) "0, 0, 0" "1,1,1") "Undefined" 0 0))
  (bind _output_get (Variables|Default|SetNewestGround _returnvalue))
  (Variables|/Game/Blueprints/BP_Ground.BP_Ground_C|SetGroundSpawner _output_get self)
  (Variables|Default|SettestSpawnPoint (Math|Vector|MakeVector (+ (.x (Variables|Default|GettestSpawnPoint)) 1.5e+02) (.y (Variables|Default|GettestSpawnPoint)) (.z (Variables|Default|GettestSpawnPoint)))))

(fn SpawnRoadReverse
  (params (ReverseStartingLoc :type Vector))
  (bind _returnvalue (Game|SpawnActorfromClass "/Game/Blueprints/BP_RoadReverse.BP_RoadReverse_C" (Math|Transform|MakeTransform (Math|Vector|MakeVector (+ (.x ReverseStartingLoc) 0.0) (- (.y ReverseStartingLoc) 1e+03) (- (.z ReverseStartingLoc) 7e+01)) "0, 0, 0" "1,1,1") "Undefined" 0 0))
  (Variables|/Game/Blueprints/BP_RoadReverse.BP_RoadReverse_C|SetRoadSpawnerReverse _returnvalue self)
  (Variables|Default|SettestSpawnPoint (Math|Vector|MakeVector (+ (.x (Variables|Default|GettestSpawnPoint)) 1.5e+02) (.y (Variables|Default|GettestSpawnPoint)) (.z (Variables|Default|GettestSpawnPoint)))))

(fn SpawnHazards
  (bind _returnvalue (Math|Random|RandomIntegerinRange 0 19))
  (bind _testspawnpoint (Variables|Default|GettestSpawnPoint))
  (if (and (>= _returnvalue 0) (< _returnvalue 5))
    (CallFunction|SpawnRoad _testspawnpoint)
    (elif (and (>= _returnvalue 5) (< _returnvalue 10))
      (CallFunction|SpawnRoadReverse _testspawnpoint)
      (elif (and (>= _returnvalue 10) (< _returnvalue 14))
        (CallFunction|SpawnWater)
        (elif (and (>= _returnvalue 14) (< _returnvalue 18))
          (CallFunction|SpawnWaterReverse)
          (elif (== _returnvalue 18)
            (CallFunction|SpawnTracks)
            (else
              (CallFunction|SpawnTracksReverse))))))))

(fn SpawnWater
  (bind _self self)
  (if (== (Math|Random|RandomIntegerinRange 0 2) 1)
    (bind _returnvalue (Game|SpawnActorfromClass "/Game/Blueprints/BP_WaterLillies.BP_WaterLillies_C" (Math|Transform|MakeTransform (Math|Vector|MakeVector (+ (.x (Variables|Default|GettestSpawnPoint)) 0.0) (- (.y (Variables|Default|GettestSpawnPoint)) 1e+02) (- (.z (Variables|Default|GettestSpawnPoint)) 8e+01)) "0, 0, 0" "1,1,1") "Undefined" 0 0))
    (Variables|/Game/Blueprints/BP_WaterLillies.BP_WaterLillies_C|SetWaterSpawner _returnvalue _self)
    (else
      (bind _returnvalue_2 (Game|SpawnActorfromClass "/Game/Blueprints/BP_Water.BP_Water_C" (Math|Transform|MakeTransform (Math|Vector|MakeVector (+ (.x (Variables|Default|GettestSpawnPoint)) 0.0) (- (.y (Variables|Default|GettestSpawnPoint)) 1e+02) (- (.z (Variables|Default|GettestSpawnPoint)) 8e+01)) "0, 0, 0" "1,1,1") "Undefined" 0 0))
      (Variables|/Game/Blueprints/BP_Water.BP_Water_C|SetWaterSpawner _returnvalue_2 _self)))
  (Variables|Default|SettestSpawnPoint (Math|Vector|MakeVector (+ (.x (Variables|Default|GettestSpawnPoint)) 1.5e+02) (.y (Variables|Default|GettestSpawnPoint)) (.z (Variables|Default|GettestSpawnPoint)))))

(fn SpawnWaterReverse
  (bind _self self)
  (if (== (Math|Random|RandomIntegerinRange 0 2) 1)
    (bind _returnvalue (Game|SpawnActorfromClass "/Game/Blueprints/BP_WaterLillies.BP_WaterLillies_C" (Math|Transform|MakeTransform (Math|Vector|MakeVector 0.0 0.0 0.0) "0, 0, 0" "1,1,1") "Undefined" 0 0))
    (Variables|/Game/Blueprints/BP_WaterLillies.BP_WaterLillies_C|SetWaterSpawner _returnvalue _self)
    (else
      (bind _returnvalue_2 (Game|SpawnActorfromClass "/Game/Blueprints/BP_WaterReverse.BP_WaterReverse_C" (Math|Transform|MakeTransform (Math|Vector|MakeVector (+ (.x (Variables|Default|GettestSpawnPoint)) 0.0) (- (.y (Variables|Default|GettestSpawnPoint)) 1e+02) (- (.z (Variables|Default|GettestSpawnPoint)) 8e+01)) "0, 0, 0" "1,1,1") "Undefined" 0 0))
      (Variables|/Game/Blueprints/BP_WaterReverse.BP_WaterReverse_C|SetWaterSpawner _returnvalue_2 _self)))
  (Variables|Default|SettestSpawnPoint (Math|Vector|MakeVector (+ (.x (Variables|Default|GettestSpawnPoint)) 1.5e+02) (.y (Variables|Default|GettestSpawnPoint)) (.z (Variables|Default|GettestSpawnPoint)))))

(fn SpawnTracks
  (bind _returnvalue (Game|SpawnActorfromClass "/Game/Blueprints/BP_Tracks.BP_Tracks_C" (Math|Transform|MakeTransform (Math|Vector|MakeVector (+ (.x (Variables|Default|GettestSpawnPoint)) 1.1e+02) (- (.y (Variables|Default|GettestSpawnPoint)) 2.2e+02) (- (.z (Variables|Default|GettestSpawnPoint)) -1e+01)) "0, 0, 0" "1,1,1") "Undefined" 0 0))
  (Variables|/Game/Blueprints/BP_Tracks.BP_Tracks_C|SetTrackSpawner _returnvalue self)
  (Variables|Default|SettestSpawnPoint (Math|Vector|MakeVector (+ (.x (Variables|Default|GettestSpawnPoint)) 1.5e+02) (.y (Variables|Default|GettestSpawnPoint)) (.z (Variables|Default|GettestSpawnPoint)))))

(fn SpawnTracksReverse
  (bind _returnvalue (Game|SpawnActorfromClass "/Game/Blueprints/BP_TracksReverse.BP_TracksReverse_C" (Math|Transform|MakeTransform (Math|Vector|MakeVector (+ (.x (Variables|Default|GettestSpawnPoint)) 1.1e+02) (- (.y (Variables|Default|GettestSpawnPoint)) 6e+02) (- (.z (Variables|Default|GettestSpawnPoint)) -1e+01)) "0, 0, 0" "1,1,1") "Undefined" 0 0))
  (Variables|/Game/Blueprints/BP_TracksReverse.BP_TracksReverse_C|SetTrackSpawner _returnvalue self)
  (Variables|Default|SettestSpawnPoint (Math|Vector|MakeVector (+ (.x (Variables|Default|GettestSpawnPoint)) 1.5e+02) (.y (Variables|Default|GettestSpawnPoint)) (.z (Variables|Default|GettestSpawnPoint)))))