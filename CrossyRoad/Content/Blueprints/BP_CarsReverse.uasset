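; BP_CarsReverse is a traffic car that moves along the world Y axis and kills the player on contact.
; Tick applies a swept offset scaled by MyCarSpeed, destroys the car below a negative Y limit, and otherwise activates its audio.
; A mesh hit on BP_Player sets IsDead and shows the restart display, guarded by Restartshowing.
; CarStopper only sets CarsCanMove, which the movement logic here never reads.
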(event OnComponentHit(StaticMesh)
  (params (HitComponent :type Primitive%20Component%20Object%20Reference) (OtherActor :type Actor%20Object%20Reference) (OtherComp :type Primitive%20Component%20Object%20Reference) (NormalImpulse :type Vector :default "0, 0, 0") (Hit :type Hit%20Result%20Structure%20%28by%20ref%29))
  (if (not (Variables|Default|Getrestartshowing))
    (bind _asbp_player (Utilities|Casting|CastToBP_Player OtherActor))
    (Variables|/Game/Blueprints/BP_Player.BP_Player_C|SetisDead _asbp_player true)
    (Default|DisplayRestart _asbp_player)
    (Variables|Default|Setrestartshowing true)))

(event EventBeginPlay)

(event Collision|EventActorBeginOverlap
  (params (OtherActor :type Actor%20Object%20Reference)))

(event EventTick
  (params (DeltaSeconds :type Float%20%28single-precision%29))
  (Transformation|AddActorWorldOffset (Math|Vector|MakeVector 0.0 (* DeltaSeconds (Variables|Default|GetMyCarSpeed)) 0.0) true)
  (if (< (.y (Transformation|GetActorLocation)) -3.5e+03)
    (Actor|DestroyActor)
    (else
      (Components|Activation|Activate (Variables|Default|GetAudio) false))))

(fn ConstructionScript)

(fn CarStopper
  (Variables|Default|SetCarsCanMove true))