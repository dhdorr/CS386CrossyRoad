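; BP_GameManager is a game manager that spawns traffic cars at a regular interval.
; Each Tick runs UpdateGame, which counts SpawnTimer down by world delta time and calls Spawncar when it expires, resetting it to DurationBetweenSpawn.
; Spawncar places a BP_Cars actor in one of three random X lanes at fixed Y and Z, with a randomly chosen car or truck mesh.
; Restart resets the spawn timer.
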(event EventBeginPlay)

(event EventTick
  (params (DeltaSeconds :type Float%20%28single-precision%29))
  (CallFunction|UpdateGame))

(fn ConstructionScript)

(fn Spawncar
  (bind _returnvalue (Game|SpawnActorfromClass "/Game/Blueprints/BP_Cars.BP_Cars_C" (Math|Transform|MakeTransform (Math|Vector|MakeVector (Math|Conversions|ToFloat(Integer) (* (Math|Random|RandomIntegerinRange -1 1) 100)) -1e+03 -5e+01) "0, 0, 0" "1,1,1") "Undefined" 0 0))
  (Components|StaticMesh|SetStaticMesh (Variables|/Game/Blueprints/BP_Cars.BP_Cars_C|GetStaticMesh _returnvalue) (Utilities|Select :Index (Math|Random|RandomIntegerinRange 0 2) :Option%200 "/Game/Voxels/car1/CS386_car1.CS386_car1" :Option%201 "/Game/Voxels/car2/cS386_car2.cS386_car2" :Option%202 "/Game/Voxels/truck1/CS386_truck.CS386_truck")))

(fn CheckSpawnTimer
  (Variables|Default|SetSpawnTimer (- (Variables|Default|GetSpawnTimer) (Utilities|Time|GetWorldDeltaSeconds)))
  (if (<= (Variables|Default|GetSpawnTimer) 0.0)
    (Variables|Default|SetSpawnTimer (Variables|Default|GetDurationBetweenSpawn))
    (CallFunction|Spawncar)))

(fn UpdateGame
  (CallFunction|CheckSpawnTimer))

(fn Restart
  (Variables|Default|SetSpawnTimer (Variables|Default|GetDurationBetweenSpawn)))