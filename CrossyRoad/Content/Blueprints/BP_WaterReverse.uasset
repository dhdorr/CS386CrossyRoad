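; BP_WaterReverse is a water lane that spawns reverse-direction logs and kills the player on contact with its Box.
; Tick runs a countdown that spawns a rotated BP_LogsReverse each time it expires; straight-log and car spawning are unused leftovers.
; Box overlap marks the player dead, shows restart and plays a splash effect once.
; Player overlaps also drive level streaming: SpawnNewZone asks WaterSpawner for new ground, and TriggerZone destroys the lane.
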(event OnComponentBeginOverlap(TriggerZone)
  (params (OverlappedComponent :type Primitive%20Component%20Object%20Reference) (OtherActor :type Actor%20Object%20Reference) (OtherComp :type Primitive%20Component%20Object%20Reference) (OtherBodyIndex :type Integer) (bFromSweep :type Boolean) (SweepResult :type Hit%20Result%20Structure%20%28by%20ref%29))
  (Utilities|Casting|CastToBP_Player OtherActor)
  (Actor|DestroyActor))

(event OnComponentBeginOverlap(Box)
  (params (OverlappedComponent :type Primitive%20Component%20Object%20Reference) (OtherActor :type Actor%20Object%20Reference) (OtherComp :type Primitive%20Component%20Object%20Reference) (OtherBodyIndex :type Integer) (bFromSweep :type Boolean) (SweepResult :type Hit%20Result%20Structure%20%28by%20ref%29))
  (if (not (Variables|Default|GetrestartShowing))
    (bind _asbp_player (Utilities|Casting|CastToBP_Player OtherActor))
    (Variables|/Game/Blueprints/BP_Player.BP_Player_C|SetisDead _asbp_player true)
    (Default|DisplayRestart _asbp_player)
    (Variables|Default|SetrestartShowing true)
    (Effects|SpawnEmitteratLocation "/Game/Blueprints/ParticleSystem/PS_Water.PS_Water" (Transformation|GetActorLocation _asbp_player))))

(event OnComponentBeginOverlap(SpawnNewZone)
  (params (OverlappedComponent :type Primitive%20Component%20Object%20Reference) (OtherActor :type Actor%20Object%20Reference) (OtherComp :type Primitive%20Component%20Object%20Reference) (OtherBodyIndex :type Integer) (bFromSweep :type Boolean) (SweepResult :type Hit%20Result%20Structure%20%28by%20ref%29))
  (bind _waterspawner (Variables|Default|GetWaterSpawner))
  (Utilities|Casting|CastToBP_Player OtherActor)
  (Utilities|IsValid _waterspawner
    (:Is%20Valid
      (Default|SpawnGroundatSpawnPoint _waterspawner))))

(event EventBeginPlay)

(event EventTick
  (params (DeltaSeconds :type Float%20%28single-precision%29))
  (CallFunction|UpdateLogs))

(event Collision|EventActorBeginOverlap
  (params (OtherActor :type Actor%20Object%20Reference))
  ;[1 1 1] Old Stuff, may reuse
)

(fn ConstructionScript)

(fn CheckSpawnTimer
  (Variables|Default|SetSpawnTimer (- (Variables|Default|GetSpawnTimer) (Utilities|Time|GetWorldDeltaSeconds)))
  (if (<= (Variables|Default|GetSpawnTimer) 0.0)
    (Variables|Default|SetSpawnTimer (Variables|Default|GetDurationBetweenSpawn))
    (CallFunction|SpawnLogs)))

(fn SpawnLogs
  (CallFunction|SpawnReverse))

(fn UpdateLogs
  (CallFunction|CheckSpawnTimer))

(fn SpawnStraight
  (bind _returnvalue (Transformation|GetActorLocation))
  (Game|SpawnActorfromClass "/Game/Blueprints/BP_Logs.BP_Logs_C" (Math|Transform|MakeTransform (Math|Vector|MakeVector (- (.x _returnvalue) -25.0) (- (.y _returnvalue) 1.5e+03) (+ (.z _returnvalue) 75.0)) "0, 0, 0" "1,1,1") "Undefined" 0 0))

(fn SpawnReverse
  (bind _returnvalue (Transformation|GetActorLocation))
  (Game|SpawnActorfromClass "/Game/Blueprints/BP_LogsReverse.BP_LogsReverse_C" (Math|Transform|MakeTransform (Math|Vector|MakeVector (- (.x _returnvalue) -25.0) 2.2e+03 (+ (.z _returnvalue) 8e+01)) "0,180.000000, 0" "1,1,1") "Undefined" 0 0))