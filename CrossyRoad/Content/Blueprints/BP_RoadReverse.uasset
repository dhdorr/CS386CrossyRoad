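; BP_RoadReverse is a road segment that periodically spawns reverse-direction cars for the player to deal with.
; Tick runs a countdown that, on expiry, randomly decides whether to spawn a rotated BP_CarsReverse at a fixed Y and gives it a random car or truck mesh.
; Player overlap with SpawnNewZone asks RoadSpawnerReverse for new ground, while overlap with TriggerZone destroys the segment.
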(event OnComponentBeginOverlap(TriggerZone)
  (params (OverlappedComponent :type Primitive%20Component%20Object%20Reference) (OtherActor :type Actor%20Object%20Reference) (OtherComp :type Primitive%20Component%20Object%20Reference) (OtherBodyIndex :type Integer) (bFromSweep :type Boolean) (SweepResult :type Hit%20Result%20Structure%20%28by%20ref%29))
  (Utilities|Casting|CastToBP_Player OtherActor)
  (Actor|DestroyActor))

(event OnComponentBeginOverlap(CarZone)
  (params (OverlappedComponent :type Primitive%20Component%20Object%20Reference) (OtherActor :type Actor%20Object%20Reference) (OtherComp :type Primitive%20Component%20Object%20Reference) (OtherBodyIndex :type Integer) (bFromSweep :type Boolean) (SweepResult :type Hit%20Result%20Structure%20%28by%20ref%29)))

(event OnComponentBeginOverlap(SpawnNewZone)
  (params (OverlappedComponent :type Primitive%20Component%20Object%20Reference) (OtherActor :type Actor%20Object%20Reference) (OtherComp :type Primitive%20Component%20Object%20Reference) (OtherBodyIndex :type Integer) (bFromSweep :type Boolean) (SweepResult :type Hit%20Result%20Structure%20%28by%20ref%29))
  (bind _roadspawnerreverse (Variables|Default|GetRoadSpawnerReverse))
  (Utilities|Casting|CastToBP_Player OtherActor)
  (Utilities|IsValid _roadspawnerreverse
    (:Is%20Valid
      (Default|SpawnGroundatSpawnPoint _roadspawnerreverse))))

(event EventBeginPlay)

(event EventTick
  (params (DeltaSeconds :type Float%20%28single-precision%29))
  (CallFunction|UpdateCars))

(event Collision|EventActorBeginOverlap
  (params (OtherActor :type Actor%20Object%20Reference))
  ;[1 1 1] Old Stuff, may reuse
)

(fn ConstructionScript)

(fn CheckSpawnTimer
  (Variables|Default|SetSpawnTimer (- (Variables|Default|GetSpawnTimer) (Utilities|Time|GetWorldDeltaSeconds)))
  (if (<= (Variables|Default|GetSpawnTimer) 0.0)
    (Variables|Default|SetSpawnTimer (Variables|Default|GetDurationBetweenSpawn))
    (CallFunction|SpawnCars)))

(fn SpawnCars
  (CallFunction|SpawnReverse))

(fn UpdateCars
  (CallFunction|CheckSpawnTimer))

(fn SpawnReverse
  (bind _returnvalue (Transformation|GetActorLocation))
  (bind _returnvalue_2 (Math|Random|RandomIntegerinRange 0 10))
  (if (and (>= _returnvalue_2 0) (< _returnvalue_2 7))
    (bind _returnvalue_3 (Game|SpawnActorfromClass "/Game/Blueprints/BP_CarsReverse.BP_CarsReverse_C" (Math|Transform|MakeTransform (Math|Vector|MakeVector (- (.x _returnvalue) -1e+02) 2.2e+03 (+ (.z _returnvalue) 2e+01)) "0,180.000000, 0" "1,1,1") "Undefined" 0 0))
    (Components|StaticMesh|SetStaticMesh (Variables|/Game/Blueprints/BP_CarsReverse.BP_CarsReverse_C|GetStaticMesh _returnvalue_3) (Utilities|Select :Index (Math|Random|RandomIntegerinRange 0 2) :Option%200 "/Game/Voxels/car1/CS386_car1.CS386_car1" :Option%201 "/Game/Voxels/car2/cS386_car2.cS386_car2" :Option%202 "/Game/Voxels/truck1/CS386_truck.CS386_truck"))))