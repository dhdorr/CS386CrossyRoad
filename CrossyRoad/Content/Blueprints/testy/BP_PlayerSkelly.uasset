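; Player pawn for a Frogger-style hopping game with car hazards, turning and hopping on directional input.
; Tick applies consumed input as a swept offset while alive, and forward/backward presses track furthest progress through Steps and BackupSteps.
; Hitting BP_Cars or BP_CarsReverse disables the hit component's collision.
; BeginPlay creates HUD and restart widgets; DisplayRestart and RestartGame toggle the restart UI, with restart resetting position, collision and death state.
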(event EventBeginPlay
  (bind _returnvalue (UserInterface|CreateWidget "/Game/UI/WBP_Restart.WBP_Restart_C"))
  (Variables|Default|SetRestartWiget _returnvalue)
  (bind _returnvalue_2 (UserInterface|CreateWidget "/Game/UI/BP_HUD.BP_HUD_C"))
  (bind _output_get (Variables|Default|SetBP_HUD _returnvalue_2))
  (UserInterface|Viewport|AddtoViewport _output_get 0))

(event Collision|EventActorBeginOverlap
  (params (OtherActor :type Actor%20Object%20Reference)))

(event EventTick
  (params (DeltaSeconds :type Float%20%28single-precision%29))
  (if (not (Variables|Default|GetisDead))
    (bind _returnvalue (Class|Pawn|ConsumeMovementInputVector))
    (Transformation|AddActorLocalOffset _returnvalue true false)))

(event Collision|EventHit
  (params (MyComp :type Primitive%20Component%20Object%20Reference) (Other :type Actor%20Object%20Reference) (OtherComp :type Primitive%20Component%20Object%20Reference) (bSelfMoved :type Boolean) (HitLocation :type Vector :default "0, 0, 0") (HitNormal :type Vector :default "0, 0, 0") (NormalImpulse :type Vector :default "0, 0, 0") (Hit :type Hit%20Result%20Structure%20%28by%20ref%29))
  (Utilities|FlowControl|Sequence
    (:then_0
      (Utilities|Casting|CastToBP_Cars Other)
      (Collision|SetCollisionEnabled MyComp "NoCollision"))
    (:then_1
      (Utilities|Casting|CastToBP_CarsReverse Other)
      (Collision|SetCollisionEnabled MyComp "NoCollision"))))

(event Input|ActionEvents|InputActionMoveForward
  (params (Key :type Key%20Structure))
  ;[1 1 1] Player Movement
  (:Pressed
    (Transformation|SetActorRotation "0,90.000000, 0")
    (Pawn|Input|AddMovementInput (* (Transformation|GetActorForwardVector) -1.0) (Variables|Default|GetHopDist) false)
    (if (< (Variables|Default|GetBackupSteps) (Variables|Default|GetSteps))
      (Math|Integer|IncrementInt (Variables|Default|GetBackupSteps))
      (else
        (bind _result (Math|Integer|IncrementInt (Variables|Default|GetSteps))
          (:%20%20
            (Variables|Default|SetBackupSteps _result)
            (Development|PrintString (Utilities|String|ToString(Float) (.z (Variables|Default|Getplayervec))))))))))

(event Input|ActionEvents|InputActionMoveBackward
  (params (Key :type Key%20Structure))
  ;[1 1 1] Player Movement
  (:Pressed
    (Transformation|SetActorRotation "0,-90.000000,0.000000")
    (Pawn|Input|AddMovementInput (Transformation|GetActorForwardVector) (Variables|Default|GetHopDist) false)
    (Math|Integer|DecrementInt (Variables|Default|GetBackupSteps))))

(event Input|ActionEvents|InputActionMoveRight
  (params (Key :type Key%20Structure))
  ;[1 1 1] Player Movement
  (:Pressed
    (Transformation|SetActorRotation "0,180.000000, 0")
    (Pawn|Input|AddMovementInput (* (Transformation|GetActorRightVector) -1.0) (* (Variables|Default|GetHopDist) -1.0) false)))

(event Input|ActionEvents|InputActionMoveLeft
  (params (Key :type Key%20Structure))
  ;[1 1 1] Player Movement
  (:Pressed
    (Transformation|SetActorRotation "0, 0, 0")
    (Pawn|Input|AddMovementInput (Transformation|GetActorRightVector) (* (Variables|Default|GetHopDist) -1.0) false)))

(fn ConstructionScript)

(fn DisplayRestart
  (bind _returnvalue (Game|GetPlayerController 0))
  (UserInterface|Viewport|AddtoViewport (Variables|Default|GetRestartWiget) 0)
  (Input|SetInputModeUIOnly _returnvalue 0 "DoNotLock")
  (Variables|/Script/Engine.PlayerController|SetbShowMouseCursor _returnvalue true))

(fn RestartGame
  (bind _returnvalue (Game|GetPlayerController 0))
  (Variables|Default|SetisDead false)
  (Widget|RemovefromParent (Variables|Default|GetRestartWiget))
  (Input|SetInputModeGameOnly _returnvalue)
  (Variables|/Script/Engine.PlayerController|SetbShowMouseCursor _returnvalue false)
  (Transformation|SetActorLocation "-460.000000,0.000000,55.000000" false false)
  (Collision|SetCollisionEnabled (Variables|Default|GetBox) "QueryAndPhysics"))